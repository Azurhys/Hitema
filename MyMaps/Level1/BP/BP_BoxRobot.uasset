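; BP_BoxRobot is a box platform in Level1 that drops after a BP_Bot touches it and then respawns.
; On BeginPlay it stores the box mesh's world transform.
; A bot overlapping the Box trigger starts a short delay, then physics is enabled on the mesh so it can fall.
; After a further delay, RespawnPlatform disables physics and teleports the mesh back to the stored transform.
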(event `self.ReceiveBeginPlay`
  (set `self.TrasnFormInit` (`SceneComponent.K2_GetComponentToWorld` (`self.BoxMesh`))))

(event `self.Box.OnComponentBeginOverlap`
  (params (OverlappedComponent :type "PrimitiveComponent Object Reference") (OtherActor :type "Actor Object Reference") (OtherComp :type "PrimitiveComponent Object Reference") (OtherBodyIndex :type Integer) (bFromSweep :type Boolean) (SweepResult :type "HitResult Structure (by ref)"))
  (cast `/Game/StackOBot/Blueprints/Character/BP_Bot` OtherActor)
  (`KismetSystemLibrary.Delay` 2.0)
  (`PrimitiveComponent.SetSimulatePhysics` (`self.BoxMesh`) true)
  (`KismetSystemLibrary.Delay` 5.0)
  (`self.RespawnPlatform`))

(event `RespawnPlatform`
  (bind _boxmesh (`self.BoxMesh`))
  (`PrimitiveComponent.SetSimulatePhysics` _boxmesh false)
  (`SceneComponent.K2_SetWorldTransform` _boxmesh (`self.TrasnFormInit`) false true))

(fn `UserConstructionScript`)